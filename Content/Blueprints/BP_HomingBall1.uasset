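; BP_HomingBall1 is a grabbable ball whose sphere continually drifts toward an actor tagged "Target".
; BeginPlay caches the transform of the last tagged actor found, so later target movement is not followed.
; Tick lerps the sphere's whole transform toward it by a fixed, frame-rate-dependent fraction.
; Grabbing only enables gravity, and bounce-counted player teleport logic is disconnected from the empty Hit event.
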(event `self.ReceiveBeginPlay`
  (bind _outactors (`GameplayStatics.GetAllActorsWithTag` "Target"))
  (for _array_element _outactors
    (set `self.Target` (`self.GetTransform` _array_element))))

(event `self.ReceiveActorBeginOverlap`
  (params (OtherActor :type "Actor Object Reference")))

(event `self.ReceiveTick`
  (params (DeltaSeconds :type "Float (single-precision)"))
  (bind _sphere (`self.Sphere`))
  (`SceneComponent.K2_SetWorldTransform` _sphere (`KismetMathLibrary.TLerp` (`SceneComponent.K2_GetComponentToWorld` _sphere) (`self.Target`) 0.01) false false))

(event `self.GrabComponent.OnGrabbed`
  ;[1 1 1] Resets teleporting when object is grabbed
  (`PrimitiveComponent.SetEnableGravity` (`self.Sphere`) true))

(event `self.ReceiveHit`
  (params (MyComp :type "PrimitiveComponent Object Reference") (Other :type "Actor Object Reference") (OtherComp :type "PrimitiveComponent Object Reference") (bSelfMoved :type Boolean) (HitLocation :type "Vector Structure") (HitNormal :type "Vector Structure") (NormalImpulse :type "Vector Structure") (Hit :type "HitResult Structure (by ref)"))
  ;[1 1 1] Collision teleport logic
)

(fn `UserConstructionScript`)