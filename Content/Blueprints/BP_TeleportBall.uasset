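; BP_TeleportBall is a grabbable ball that teleports the player to where it lands after being thrown.
; Grabbing it resets the bounce count, re-arms teleporting and turns on gravity for the sphere.
; While released, each hit on a Floor-tagged actor increments and prints the count until it equals the bounce limit, when that hit moves the player pawn to the impact point and disarms the ball.
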(event `self.ReceiveBeginPlay`)

(event `self.ReceiveActorBeginOverlap`
  (params (OtherActor :type "Actor Object Reference")))

(event `self.GrabComponent.OnGrabbed`
  ;[1 1 1] Resets teleporting when object is grabbed
  (set `self.BounceCounter` 0)
  (set `self.CanTeleportPlayer` true)
  (`PrimitiveComponent.SetEnableGravity` (`self.Sphere`) true))

(event `self.ReceiveHit`
  (params (MyComp :type "PrimitiveComponent Object Reference") (Other :type "Actor Object Reference") (OtherComp :type "PrimitiveComponent Object Reference") (bSelfMoved :type Boolean) (HitLocation :type "Vector Structure") (HitNormal :type "Vector Structure") (NormalImpulse :type "Vector Structure") (Hit :type "HitResult Structure (by ref)"))
  ;[1 1 1] Collision teleport logic
  (if (`self.CanTeleportPlayer`)
    (if (`/Game/VRTemplate/Blueprints/GrabComponent.bIsHeld` (`self.GrabComponent`))
      _
      (elif (`self.ActorHasTag` Other "Floor")
        (if (== (`self.BounceCounter`) (`self.BounceLimit`))
          (`self.K2_SetActorLocation` (`GameplayStatics.GetPlayerPawn` 0) HitLocation false false)
          (set `self.CanTeleportPlayer` false)
          (else
            (bind _result (`/Engine/EditorBlueprintResources/StandardMacros.IncrementInt` (`self.BounceCounter`))
              (:`  `
                (`KismetSystemLibrary.PrintString` (`KismetStringLibrary.Conv_IntToString` _result))))))))))

(fn `UserConstructionScript`)