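; BP_Taro is a greenhouse taro plant that gradually dries out and is refreshed by a watering can.
; Each Tick pushes the Dryness value to the plant mesh materials as a scalar parameter, then raises it by a fixed per-frame step up to a cap, printing it for debugging.
; An actor tagged WateringCan overlapping the Pot component resets Dryness to zero.
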(event `self.ReceiveTick`
  (params (DeltaSeconds :type "Float (single-precision)"))
  (bind _dryness (`self.Dryness`))
  (`MeshComponent.SetScalarParameterValueOnMaterials` (`self.SM_Plant_Taro_01`) "Dryness" _dryness)
  (if (< _dryness 1.0)
    (set `self.Dryness` (+ _dryness 0.01))
    (`KismetSystemLibrary.PrintString` (`KismetStringLibrary.Conv_DoubleToString` _dryness))))

(event `self.Pot.OnComponentBeginOverlap`
  (params (OverlappedComponent :type "PrimitiveComponent Object Reference") (OtherActor :type "Actor Object Reference") (OtherComp :type "PrimitiveComponent Object Reference") (OtherBodyIndex :type Integer) (bFromSweep :type Boolean) (SweepResult :type "HitResult Structure (by ref)"))
  (if (`self.ActorHasTag` OtherActor "WateringCan")
    (set `self.Dryness` 0.0)))

(fn `UserConstructionScript`)