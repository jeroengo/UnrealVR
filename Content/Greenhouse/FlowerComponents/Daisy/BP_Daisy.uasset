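; BP_Daisy is a greenhouse daisy that tracks how dry its pot is as a 0 to 1 value, exposed through GetPotDryness.
; An actor tagged WateringCan overlapping the Pot toggles watering, as does holding Y, which also prints a message.
; Each tick lerps dryness toward wet while watering and more slowly toward dry otherwise, using fixed alphas that make the rate frame-dependent.
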(event `self.ReceiveTick`
  (params (DeltaSeconds :type "Float (single-precision)"))
  (bind _potdryness (`self.PotDryness`))
  (if (`self.bIsWatering`)
    (set `self.PotDryness` (`KismetMathLibrary.Lerp` _potdryness 0.0 0.05))
    (elif (< _potdryness 1.0)
      (set `self.PotDryness` (`KismetMathLibrary.Lerp` _potdryness 1.0 0.005)))))

(event `self.Pot.OnComponentBeginOverlap`
  (params (OverlappedComponent :type "PrimitiveComponent Object Reference") (OtherActor :type "Actor Object Reference") (OtherComp :type "PrimitiveComponent Object Reference") (OtherBodyIndex :type Integer) (bFromSweep :type Boolean) (SweepResult :type "HitResult Structure (by ref)"))
  (if (`self.ActorHasTag` OtherActor "WateringCan")
    (set `self.bIsWatering` true :!label _label)))

(event `Key|Y`
  (params (Key :type "Key Structure"))
  (:`Pressed`
    (`KismetSystemLibrary.PrintString` "Watering")
    (goto _label))
  (:`Released`
    (set `self.bIsWatering` false :!label _label_2)))

(event `self.Pot.OnComponentEndOverlap`
  (params (OverlappedComponent :type "PrimitiveComponent Object Reference") (OtherActor :type "Actor Object Reference") (OtherComp :type "PrimitiveComponent Object Reference") (OtherBodyIndex :type Integer))
  (if (`self.ActorHasTag` OtherActor "WateringCan")
    (goto _label_2)))

(fn `GetPotDryness`
  (returns (PotDryness :type "Float (double-precision)"))
  (return (`self.PotDryness`)))

(fn `UserConstructionScript`)