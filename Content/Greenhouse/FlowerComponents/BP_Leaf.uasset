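; Greenhouse flower leaf actor that grows, shows dryness and can be plucked by grabbing.
; While connected, a BeginPlay timeline drives the mesh scale and Tick pushes LeafDryness into the material's Dryness parameter.
; Grabbing disconnects and detaches the leaf, freezing both updates, and dropping it turns on physics.
; A debug R key disconnects it and enables physics without detaching the actor.
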(event OnGrabbed(GrabComponent)
  (Variables|Default|SetIsConnected false)
  (Transformation|DetachFromActor "KeepRelative" "KeepRelative" "KeepRelative")
  (Development|PrintString "Detatching"))

(event OnDropped(GrabComponent)
  (Physics|SetSimulatePhysics (Variables|Default|GetLeaf) true))

(event EventBeginPlay
  (bind _growth (Timeline|Timeline Play)
    (:Update
      (if (Variables|Default|GetIsConnected)
        (Transformation|SetRelativeScale3D (Variables|Default|GetLeaf) _growth)))))

(event Collision|EventActorBeginOverlap
  (params (OtherActor :type Actor%20Object%20Reference)))

(event EventTick
  (params (DeltaSeconds :type Float%20%28single-precision%29))
  (if (Variables|Default|GetIsConnected)
    (Rendering|Material|SetScalarParameterValueonMaterials (Variables|Default|GetLeaf) "Dryness" (Variables|Default|GetLeafDryness))))

(event Input|KeyboardEvents|DebugKeyR
  (params (Key :type Key%20Structure :default "None") (ActionValue :type Input%20Action%20Value%20Structure))
  (:Pressed
    (Variables|Default|SetIsConnected false)
    (Physics|SetSimulatePhysics (Variables|Default|GetLeaf) true)))

(fn ConstructionScript)