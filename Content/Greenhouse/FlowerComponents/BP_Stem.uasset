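; BP_Stem is a greenhouse plant stem that grows leaves and flowers and shows the pot's dryness.
; BeginPlay finds the BP_GrowingPlant as its pot, spawns leaves and flowers attached to anchor components, and scales the stem via timeline.
; A T debug key repeats the spawning.
; Tick passes pot dryness to flowers, leaves and the stem material, with leaf and stem updates nested inside the flower loop.
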(event EventTick
  (params (DeltaSeconds :type Float%20%28single-precision%29))
  (bind _potdryness (Default|GetPotDryness (Variables|Default|GetPot)))
  (for _array_element (Variables|Default|GetSpawnedFlowers)
    (Utilities|IsValid _array_element
      (:Is%20Valid
        (Variables|/Game/Greenhouse/FlowerComponents/BP_Flower.BP_Flower_C|SetFlowerDryness _array_element _potdryness))
      (:Is%20Not%20Valid
        _))
    (for _array_element_2 (Variables|Default|GetSpawnedLeaves)
      (Utilities|IsValid _array_element_2
        (:Is%20Valid
          (Variables|/Game/Greenhouse/FlowerComponents/BP_Leaf.BP_Leaf_C|SetLeafDryness _array_element_2 _potdryness))
        (:Is%20Not%20Valid
          _))
      (Rendering|Material|SetScalarParameterValueonMaterials (Variables|Default|GetStem) "Dryness" _potdryness))))

(event EventBeginPlay
  (bind _returnvalue (Actor|GetActorOfClass "/Game/Greenhouse/FlowerComponents/BP_GrowingPlant.BP_GrowingPlant_C"))
  (Variables|Default|SetPot _returnvalue)
  (Utilities|FlowControl|Sequence
    (:then_0
      (bind _output_get (Variables|Default|SetLeafAnchors (Utilities|Array|MakeArray (Variables|Default|GetLeafAnchor) (Variables|Default|GetLeafAnchor1))))
      (for _array_element _output_get
        (CallFunction|SpawnLeaf _array_element)))
    (:then_1
      (bind _output_get_2 (Variables|Default|SetFlowerAnchors (Utilities|Array|MakeArray (Variables|Default|GetFlowerAnchor) (Variables|Default|GetFlowerAnchor1))))
      (for _array_element_2 _output_get_2
        (CallFunction|SpawnFlower _array_element_2)))
    (:then_2
      (bind _scaletrack (Timeline|Timeline_0 Play)
        (:Update
          (Transformation|SetWorldScale3D (Variables|Default|GetStem) _scaletrack))))))

(event Input|KeyboardEvents|DebugKeyT
  (params (Key :type Key%20Structure :default "None") (ActionValue :type Input%20Action%20Value%20Structure))
  (:Pressed
    (Utilities|FlowControl|Sequence
      (:then_0
        (for _array_element (stale EventBeginPlay _output_get)
          (CallFunction|SpawnLeaf _array_element)))
      (:then_1
        (for _array_element_2 (stale EventBeginPlay _output_get_2)
          (CallFunction|SpawnFlower _array_element_2))))))

(fn ConstructionScript)

(fn SpawnLeaf
  (params (Anchor :type Arrow%20Component%20Object%20Reference))
  (Development|PrintString "Adding Leaf")
  (bind _returnvalue (Game|SpawnActorfromClass "/Game/Greenhouse/FlowerComponents/BP_Leaf.BP_Leaf_C" (Transformation|GetRelativeTransform Anchor) "Undefined" "MultiplyWithRoot" 0 0))
  (Utilities|Array|Add (Variables|Default|GetSpawnedLeaves) _returnvalue)
  (Utilities|IsValid _returnvalue
    (:Is%20Valid
      (Transformation|AttachComponentToComponent _returnvalue Anchor "None" "SnapToTarget" "SnapToTarget" "SnapToTarget" false))))

(fn SpawnFlower
  (params (Anchor :type Arrow%20Component%20Object%20Reference))
  (Development|PrintString "Adding Flower")
  (bind _returnvalue (Game|SpawnActorfromClass "/Game/Greenhouse/FlowerComponents/BP_Flower.BP_Flower_C" (Transformation|GetRelativeTransform Anchor) "Undefined" "MultiplyWithRoot" 0 0))
  (Utilities|Array|Add (Variables|Default|GetSpawnedFlowers) _returnvalue)
  (Utilities|IsValid _returnvalue
    (:Is%20Valid
      (Transformation|AttachComponentToComponent _returnvalue Anchor "None" "SnapToTarget" "SnapToTarget" "SnapToTarget" false))))