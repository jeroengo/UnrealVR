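; Greenhouse plant actor that animates its growth when play begins.
; A Timeline scales the stem on one track, and the flower and two cached leaves on a shared leaf track.
; In parallel, a five-second delay prints a debug string, destroys the BPLeaf component, then spawns a BP_Leaf actor at LeafAnchor3's relative transform and attaches it to the plant.
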(event `self.ReceiveBeginPlay`
  (set `self.Leaves` (`|MakeArray` (`self.Leaf1`) (`self.Leaf2`)))
  (`|ExecutionSequence`
    (:`then_0`
      (bind (_direction _scaletrack _leafscale) (`Timeline|Timeline`)
        (:`Update`
          (`SceneComponent.SetWorldScale3D` (`self.Stem`) _scaletrack)
          (`SceneComponent.SetWorldScale3D` (`self.Flower`) _leafscale)
          (for _array_element (`self.Leaves`)
            (`SceneComponent.SetWorldScale3D` _array_element _leafscale)))))
    (:`then_1`
      (`KismetSystemLibrary.Delay` 5.0)
      (`KismetSystemLibrary.PrintString` "Hello")
      (`ActorComponent.K2_DestroyComponent` (`self.BP_Leaf`))
      (bind _returnvalue (`|SpawnActorFromClass` "/Game/Greenhouse/BP_Leaf.BP_Leaf_C" (`SceneComponent.GetRelativeTransform` (`self.LeafAnchor3`)) "Undefined" "MultiplyWithRoot" null null))
      (`self.K2_AttachToActor` _returnvalue self "None" "KeepRelative" "KeepRelative" "KeepRelative" true))))

(fn `UserConstructionScript`)