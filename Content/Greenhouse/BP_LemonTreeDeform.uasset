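; Lemon tree actor for the greenhouse that dries out over time, bending its mesh via Geometry Script.
; Construction copies InputMesh and its first material into a DynamicMeshComponent.
; Tick feeds Dryness to the material and, until it reaches one, increments it and bends the already-deformed mesh with a Dryness-scaled extent.
; A WateringCan-tagged overlap on Pot resets Dryness and applies a zero bend, without re-copying the mesh.
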(event `self.Pot.OnComponentBeginOverlap`
  (params (OverlappedComponent :type "PrimitiveComponent Object Reference") (OtherActor :type "Actor Object Reference") (OtherComp :type "PrimitiveComponent Object Reference") (OtherBodyIndex :type Integer) (bFromSweep :type Boolean) (SweepResult :type "HitResult Structure (by ref)"))
  (`KismetSystemLibrary.PrintString` "Overlap")
  (if (`self.ActorHasTag` OtherActor "WateringCan")
    (`KismetSystemLibrary.PrintString` "Hello")
    (set `self.Dryness` 0.0)
    (`GeometryScriptLibrary_MeshDeformFunctions.ApplyBendWarpToMesh` (`self.Dynamic Mesh`) (struct) (struct) 0.0 0.0 null)))

(event `self.ReceiveTick`
  (params (DeltaSeconds :type "Float (single-precision)"))
  (bind _dryness (`self.Dryness`))
  (`MeshComponent.SetScalarParameterValueOnMaterials` (`self.DynamicMeshComponent`) "Dryness" _dryness)
  (if (< _dryness 1.0)
    (set `self.Dryness` (+ _dryness 0.001))
    (`KismetSystemLibrary.PrintString` (`KismetStringLibrary.Conv_DoubleToString` _dryness))
    (`GeometryScriptLibrary_MeshDeformFunctions.ApplyBendWarpToMesh` (`self.Dynamic Mesh`) (struct) (struct) (`self.BendAngle`) (* (`self.Dryness`) (`self.BendExtent`)) null)))

(fn `UserConstructionScript`
  (bind _inputmesh (`self.InputMesh`))
  (bind _returnvalue (`BaseDynamicMeshComponent.GetDynamicMesh` (`self.DynamicMeshComponent`)))
  (bind _returnvalue_2 (`GeometryScriptLibrary_StaticMeshFunctions.CopyMeshFromStaticMesh` _inputmesh _returnvalue (struct) (struct) null)
    (:`Success`
      (set `self.Dynamic Mesh` _returnvalue_2)
      (`PrimitiveComponent.SetMaterial` (`self.DynamicMeshComponent`) 0 (`StaticMesh.GetMaterial` _inputmesh 0)))))